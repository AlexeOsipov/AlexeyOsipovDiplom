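; BP_Line is an actor that adds and removes a "line" mesh using a configurable mesh, color and scale.
; BeginPlay applies the mesh to its StaticMesh; CreateLine spawns a second mesh component at that world transform, with a dynamic MAT_LINE_Inst material fed Color and Scale.
; DeleteLine destroys that component but sets HasLine to true, so the HasLine guard blocks any later CreateLine.
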(event Custom|Create%20Line
  (if (not (Variables|Default|GetHas%20Line))
    (bind _returnvalue (AddComponent|AddStaticMeshComponent true (Transformation|GetWorldTransform (Variables|Default|GetStaticMesh))))
    (bind _output_get (Variables|Default|SetMesh_Component _returnvalue))
    (Components|StaticMesh|SetStaticMesh _output_get (Variables|Default|GetMesh))
    (bind _returnvalue_2 (Rendering|Material|CreateDynamicMaterialInstance _output_get 0 "/Game/Materialsline/MAT_LINE_Inst.MAT_LINE_Inst" "None" :!class /Script/Engine.PrimitiveComponent))
    (Rendering|Material|SetVectorParameterValue _returnvalue_2 "Color" (Variables|Default|GetColor) :!class /Script/Engine.MaterialInstanceDynamic)
    (Rendering|Material|SetScalarParameterValue _returnvalue_2 "Scale" (Variables|Default|GetScale) :!class /Script/Engine.MaterialInstanceDynamic)
    (Variables|Default|SetHas%20Line true)))

(event Custom|Delete%20Line
  (bind _mesh_component (Variables|Default|GetMesh_Component))
  (Utilities|IsValid _mesh_component
    (:Is%20Valid
      (Components|DestroyComponent _mesh_component)
      (Variables|Default|SetHas%20Line true))))

(event EventBeginPlay
  (Components|StaticMesh|SetStaticMesh (Variables|Default|GetStaticMesh) (Variables|Default|GetMesh)))

(event Collision|EventActorBeginOverlap
  (params (OtherActor :type Actor%20Object%20Reference)))

(event EventTick
  (params (DeltaSeconds :type Float%20%28single-precision%29)))

(fn ConstructionScript)